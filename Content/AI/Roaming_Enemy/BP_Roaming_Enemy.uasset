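; BP_Roaming_Enemy is a roaming AI enemy character that can walk, run and fire projectiles.
; Walk and Run events switch its movement speed, while Attack plays a one-shot animation, sets Attacking and, after a delay, spawns a BP_FirstPersonProjectile along its control rotation.
; An unconnected line-trace hit check holds the only Attacking reset and return to Animation Blueprint mode, so neither runs.
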(event `Walk`
  (set `CharacterMovementComponent.MaxWalkSpeed` 180.0 (`self.CharacterMovement`)))

(event `Run`
  (set `CharacterMovementComponent.MaxWalkSpeed` 350.0 (`self.CharacterMovement`)))

(event `Attack`
  (bind (_returnvalue_x _returnvalue_y _returnvalue_z) (`KismetMathLibrary.BreakVector` (`self.K2_GetActorLocation`)))
  (`SkeletalMeshComponent.PlayAnimation` (`self.Mesh`) null false)
  (set `self.Attacking` true)
  (`KismetSystemLibrary.Delay` 1.5)
  (`|SpawnActorFromClass` "/Game/FirstPerson/Blueprints/BP_FirstPersonProjectile.BP_FirstPersonProjectile_C" (`KismetMathLibrary.MakeTransform` (`KismetMathLibrary.MakeVector` _returnvalue_x _returnvalue_y (+ _returnvalue_z 60.0)) (`self.GetControlRotation`)) "AlwaysSpawn" "MultiplyWithRoot" null null))

(fn `UserConstructionScript`)